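; A one-shot interactable door that opens in two dramatic stages with pauses between them.
; InteractPressed sets InteractState, then after a short delay a timeline slides the door to a first end position, and after another pause a second timeline moves it to the final one.
; BeginPlay applies DoorRate to both timelines, and InteractQueried reports InteractState.
; The state reset is unconnected, so the door never re-arms.
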(event `self.ReceiveBeginPlay`
  (bind _door_rate (`self.Door Rate`))
  (bind _output_get (set `self.TM_Door_Animation` (`self.TM_Door_Animation`)))
  (`TimelineComponent.SetPlayRate` _output_get _door_rate)
  (`TimelineComponent.SetPlayRate` (`self.TM_Dramatic_Door`) _door_rate))

(event `self.Interact_Pressed`
  (if (not (`self.Interact_State`))
    (set `self.Interact_State` true)
    (`KismetSystemLibrary.Delay` 0.5)
    (bind (_direction _alpha) (`Timeline|TM_Door_Animation`)
      (:`Update`
        (`SceneComponent.K2_SetRelativeLocation` (`self.Door`) (`KismetMathLibrary.VLerp` (`self.Start_Location`) (`self.End_Location1`) _alpha) false false))
      (:`Finished`
        (`KismetSystemLibrary.Delay` 1.0)
        (bind (_direction_2 _alpha_2) (`Timeline|TM_Dramatic_Door`)
          (:`Update`
            (`SceneComponent.K2_SetRelativeLocation` (`self.Door`) (`KismetMathLibrary.VLerp` (`self.End_Location1`) (`self.End_Location2`) _alpha_2) false false)))))))

(fn `Interact_Queried`
  (returns (Trace_Result :type Boolean))
  (return (`self.Interact_State`)))

(fn `UserConstructionScript`)