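; BP_Sphere_Interact is an interactable sphere actor that changes color in response to interaction and overlap.
; InteractPressed toggles the TraceResult boolean, swapping the sphere's material to green when true and solid blue when false.
; Overlap by a BP_Penny actor turns the sphere red without altering TraceResult.
; InteractQueried returns TraceResult so other objects can read the toggle state.
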(event `self.ReceiveActorBeginOverlap`
  (params (OtherActor :type "Actor Object Reference"))
  (cast `/Game/Blueprints/BP_Penny` OtherActor)
  (`PrimitiveComponent.SetMaterial` (`self.Sphere`) 0 "/Game/Materials/M_Red_Inst.M_Red_Inst"))

(event `/Game/Blueprints/BPIs/i_Interactable.Interact_Pressed`
  (if (`self.Trace Result`)
    (set `self.Trace Result` false)
    (`PrimitiveComponent.SetMaterial` (`self.Sphere`) 0 "/Game/LevelPrototyping/Materials/MI_Solid_Blue.MI_Solid_Blue")
    (else
      (set `self.Trace Result` true)
      (`PrimitiveComponent.SetMaterial` (`self.Sphere`) 0 "/Game/Materials/M_Green_Inst.M_Green_Inst"))))

(fn `Interact_Queried`
  (returns (Trace_Result :type Boolean))
  (return (`self.Trace Result`)))

(fn `UserConstructionScript`)