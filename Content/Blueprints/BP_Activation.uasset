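; BP_Activation is a trigger box that activates tagged platforms when the player walks in holding a key.
; On BeginPlay it caches every BP_Platform_Base actor in the level, avoiding repeated world searches.
; On box overlap it casts to BP_ThirdPersonCharacter_Lo and checks HasKey, then a DoOnce calls EvActivate on each cached platform matching its Tag, so it fires only once.
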(event `self.ReceiveBeginPlay`
  ; Very expensive! Thankfully, this is run once on load time, so it is thoughtful
  (bind _outactors (`GameplayStatics.GetAllActorsOfClass` "/Game/Blueprints/BP_Platform_Base.BP_Platform_Base_C"))
  (set `self.Platform_Ref` _outactors))

(event `self.Box.OnComponentBeginOverlap`
  (params (OverlappedComponent :type "PrimitiveComponent Object Reference") (OtherActor :type "Actor Object Reference") (OtherComp :type "PrimitiveComponent Object Reference") (OtherBodyIndex :type Integer) (bFromSweep :type Boolean) (SweepResult :type "HitResult Structure (by ref)"))
  ; It is saying, can we convert this actor into a BP_Third_Person_Character_Lo? If yes, act as it!
  (bind _asbp_third_person_character_lo (cast `/Game/ThirdPerson/Blueprints/BP_ThirdPersonCharacter_Lo` OtherActor))
  (if (`/Game/ThirdPerson/Blueprints/BP_ThirdPersonCharacter_Lo.Has_Key` _asbp_third_person_character_lo)
    (`/Engine/EditorBlueprintResources/StandardMacros.DoOnce` false
      (:`Completed`
        (for _array_element (`self.Platform_Ref`)
          (if (`self.ActorHasTag` _array_element (`self.Tag`))
            (`/Game/Blueprints/BP_Platform_Base.Ev Activate` _array_element)))))))

(fn `UserConstructionScript`)