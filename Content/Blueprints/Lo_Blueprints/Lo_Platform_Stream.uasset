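; Floating ice platform that drifts downstream along a stream, sinks and respawns at its start point on a repeating cycle.
; BeginPlay caches the start position, derives submerged positions from Depth, sets timeline play rates and starts the cycle.
; A downstream timeline lerps the mesh to StreamEnd after a delay, then a sink timeline lowers it and snaps it back.
; The forward event re-arms itself through a RespawnTime timer.
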(event `Ev Sink`
  (bind (_direction _alpha) (`Timeline|TM_Sink` :!via `PlayFromStart`)
    (:`Update`
      (`SceneComponent.K2_SetRelativeLocation` (`self.Platform`) (`KismetMathLibrary.VLerp` (`self.Stream_End`) (`self.Submerge_End`) _alpha) false false))
    (:`Finished`
      (`SceneComponent.K2_SetRelativeLocation` (`self.Platform`) (`self.Stream_Start`) false false))))

(event `Ev Platform Forward`
  (`KismetSystemLibrary.K2_SetTimerDelegate` (delegate `Ev Platform Forward`) (`self.Respawn_Time`) true)
  (`KismetSystemLibrary.Delay` (`self.Start_Delay`))
  (bind (_direction _alpha) (`Timeline|TM_Downstream` :!via `PlayFromStart`)
    (:`Update`
      (`SceneComponent.K2_SetRelativeLocation` (`self.Platform`) (`KismetMathLibrary.VLerp` (`self.Stream_Start`) (`self.Stream_End`) _alpha) false false))
    (:`Finished`
      (`KismetSystemLibrary.Delay` (`self.End_Delay`))
      (`self.Ev Sink`))))

(event `self.ReceiveBeginPlay`
  (bind (_stream_end_x _stream_end_y _stream_end_z) (`KismetMathLibrary.BreakVector` (`self.Stream_End`)))
  (bind _output_get (set `self.Stream_Start` (`SceneComponent.RelativeLocation` (`self.Platform`))))
  (set `self.Submerge_Start` (`KismetMathLibrary.MakeVector` (.x _output_get) (.y _output_get) (- (.z _output_get) (`self.Depth`))))
  (set `self.Submerge_End` (`KismetMathLibrary.MakeVector` _stream_end_x _stream_end_y (- _stream_end_z (`self.Depth`))))
  (`TimelineComponent.SetPlayRate` (`self.TM_Downstream`) (`self.Stream_Rate`))
  (`TimelineComponent.SetPlayRate` (`self.TM_Sink`) (`self.Sink_Rate`))
  (`self.Ev Platform Forward`))

(fn `UserConstructionScript`
  (`StaticMeshComponent.SetStaticMesh` (`self.Platform`) "/Game/Static_Meshes/Floating_Ice.Floating_Ice"))