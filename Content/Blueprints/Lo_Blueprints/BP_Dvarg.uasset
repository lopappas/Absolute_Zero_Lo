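; BP_Dvarg is a Dvarg actor built from a sphere body and three cylinders for legs, with configurable colors.
; Its construction script reads the DvargAesthetics settings, which choose separately for legs and body between a specified material and a random pick from a list.
; All three cylinders share the chosen leg material, while the sphere takes the body material.
; The event graph holds no active logic.
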(fn `UserConstructionScript`
  (bind (_legcolor _bodycolor _legmethod _bodymethod _legcolorlist _bodycolorlist) (break `/Game/Blueprints/Lo_Blueprints/Struct_Dvarg_Aesthetic` (`self.Dvarg_Aesthetics`)))
  (switch `/Game/Blueprints/Enums_Structs/Enum_Color_Options` _legmethod
    (:`NewEnumerator0`
      (`PrimitiveComponent.SetMaterial` (`self.Cylinder`) 0 _legcolor)
      (`PrimitiveComponent.SetMaterial` (`self.Cylinder1`) 0 _legcolor)
      (`PrimitiveComponent.SetMaterial` (`self.Cylinder2`) 0 _legcolor))
    (:`NewEnumerator1`
      (`PrimitiveComponent.SetMaterial` (`self.Cylinder`) 0 (`KismetArrayLibrary.Array_Random` _legcolorlist))
      (`PrimitiveComponent.SetMaterial` (`self.Cylinder1`) 0 (`KismetArrayLibrary.Array_Random` _legcolorlist))
      (`PrimitiveComponent.SetMaterial` (`self.Cylinder2`) 0 (`KismetArrayLibrary.Array_Random` _legcolorlist))))
  (switch `/Game/Blueprints/Enums_Structs/Enum_Color_Options` _bodymethod
    (:`NewEnumerator0`
      (`PrimitiveComponent.SetMaterial` (`self.Sphere`) 0 _bodycolor))
    (:`NewEnumerator1`
      (`PrimitiveComponent.SetMaterial` (`self.Sphere`) 0 (`KismetArrayLibrary.Array_Random` _bodycolorlist)))))