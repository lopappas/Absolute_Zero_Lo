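; BP_Lo_Leet is an actor that keeps swapping the material on its Cube to a random entry from a material instance list.
; A custom event sets the random material, waits for RandomizeDelay, then calls itself to loop indefinitely from BeginPlay.
; BeginPlay also builds a list of the material display names through a helper function, then iterates it without acting on the entries.
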(event `self.ReceiveBeginPlay`
  (bind _output_material_inst_name_list (`self.Fn_Material_Inst_Name_List` (`self.Material_Inst_List`)))
  (bind _output_get (set `self.Output Material Inst Name List` _output_material_inst_name_list))
  (for _ _output_get
    _)
  (`self.EV Randomize_Material`))

(event `EV Randomize_Material`
  (`PrimitiveComponent.SetMaterial` (`self.Cube`) 0 (`KismetArrayLibrary.Array_Random` (`self.Material_Inst_List`)))
  (`KismetSystemLibrary.Delay` (`self.Randomize_Delay`))
  (`self.EV Randomize_Material`))

(event `self.ReceiveTick`
  (params (DeltaSeconds :type "Float (single-precision)")))

(fn `Fn_Material_Inst_Name_List`
  (params (Input_Material_Inst_List :type "Array of MaterialInstance Object Reference"))
  (returns (Output_Material_Inst_Name_List :type "Array of String"))
  (locals (Local_Material_Inst_List :type "Array of MaterialInstance Object Reference") (Counter :type Integer) (Local_Material_Inst_Name_List :type "Array of String"))
  (bind _local_material_inst_name_list (`local.Local_Material_Inst_Name_List`))
  (while (< (`local.Counter`) (`KismetArrayLibrary.Array_Length` Input_Material_Inst_List))
    (`KismetArrayLibrary.Array_Add` _local_material_inst_name_list (`KismetSystemLibrary.GetDisplayName` (`|GetArrayItem` Input_Material_Inst_List (`local.Counter`))))
    (`/Engine/EditorBlueprintResources/StandardMacros.IncrementInt` (`local.Counter`)))
  (return _local_material_inst_name_list))

(fn `UserConstructionScript`)