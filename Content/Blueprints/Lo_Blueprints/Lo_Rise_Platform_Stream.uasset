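; Actor for a floating ice platform that rises, travels downstream and sinks in a repeating cycle.
; Three timelines lerp the platform's relative location in sequence for float, downstream and sink, with configurable delays around the downstream leg.
; BeginPlay derives the submerged end from a depth offset, applies per-phase play rates and starts the cycle.
; A timer set in the float event restarts it at a fixed interval, independent of the sink finishing.
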(event `Ev Float`
  (`KismetSystemLibrary.K2_SetTimerDelegate` (delegate `Ev Float`) 25.0 true)
  (bind (_direction _alpha) (`Timeline|TM_Float` :!via `PlayFromStart`)
    (:`Update`
      (`SceneComponent.K2_SetRelativeLocation` (`self.Platform`) (`KismetMathLibrary.VLerp` (`self.Submerge_Start`) (`self.Stream_Start`) _alpha) false false))
    (:`Finished`
      (`KismetSystemLibrary.Delay` (`self.Start_Delay`))
      (`self.Ev Platform Forward`))))

(event `Ev Sink`
  (bind (_direction _alpha) (`Timeline|TM_Sink` :!via `PlayFromStart`)
    (:`Update`
      (`SceneComponent.K2_SetRelativeLocation` (`self.Platform`) (`KismetMathLibrary.VLerp` (`self.Stream_End`) (`self.Submerge_End`) _alpha) false false))))

(event `Ev Platform Forward`
  (bind (_direction _alpha) (`Timeline|TM_Downstream` :!via `PlayFromStart`)
    (:`Update`
      (`SceneComponent.K2_SetRelativeLocation` (`self.Platform`) (`KismetMathLibrary.VLerp` (`self.Stream_Start`) (`self.Stream_End`) _alpha) false false))
    (:`Finished`
      (`KismetSystemLibrary.Delay` (`self.End_Delay`))
      (`self.Ev Sink`))))

(event `self.ReceiveBeginPlay`
  (bind (_stream_end_x _stream_end_y _stream_end_z) (`KismetMathLibrary.BreakVector` (`self.Stream_End`)))
  (set `self.Stream_Start` (`SceneComponent.RelativeLocation` (`self.Platform`)))
  (set `self.Submerge_End` (`KismetMathLibrary.MakeVector` _stream_end_x _stream_end_y (- _stream_end_z (`self.Depth`))))
  (`TimelineComponent.SetPlayRate` (`self.TM_Downstream`) (`self.Stream_Rate`))
  (`TimelineComponent.SetPlayRate` (`self.TM_Sink`) (`self.Sink_Rate`))
  (`TimelineComponent.SetPlayRate` (`self.TM_Float`) (`self.Rise_Rate`))
  (`self.Ev Float`))

(fn `UserConstructionScript`
  (`StaticMeshComponent.SetStaticMesh` (`self.Platform`) "/Game/Static_Meshes/Floating_Ice.Floating_Ice"))