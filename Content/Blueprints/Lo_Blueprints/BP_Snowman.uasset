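; BP_Snowman is a snowman actor with configurable materials for its body, face and buttons, and arms.
; The construction script reads the ColorProperties struct to apply either specific materials or random picks from per-part lists.
; EvRandomize re-rolls those random materials on demand.
; The first hit on the Base plays a 2D explosion sound if it comes from BP_ThirdPersonCharacter_Lo; DoOnce precedes the cast, so any first hit consumes it.
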(event `Ev Randomize`
  (bind (_coloroptions _snowcolor _armcolor _buttoncolor _snowcolorlist _armcolorlist _buttoncolorlist) (break `/Game/Blueprints/Enums_Structs/Struct_Snowman_Color_Properties` (`self.Color_Properties`)))
  (`PrimitiveComponent.SetMaterial` (`self.Base`) 0 (`KismetArrayLibrary.Array_Random` _snowcolorlist))
  (`PrimitiveComponent.SetMaterial` (`self.Abdomin`) 0 (`KismetArrayLibrary.Array_Random` _snowcolorlist))
  (`PrimitiveComponent.SetMaterial` (`self.Head`) 0 (`KismetArrayLibrary.Array_Random` _snowcolorlist))
  (`PrimitiveComponent.SetMaterial` (`self.Snow_Face2`) 0 (`KismetArrayLibrary.Array_Random` _buttoncolorlist))
  (`PrimitiveComponent.SetMaterial` (`self.Snowman_Buttons`) 0 (`KismetArrayLibrary.Array_Random` _buttoncolorlist))
  (`PrimitiveComponent.SetMaterial` (`self.Snowman_Arms`) 0 (`KismetArrayLibrary.Array_Random` _armcolorlist))
  (`PrimitiveComponent.SetMaterial` (`self.Snowman_Arms1`) 0 (`KismetArrayLibrary.Array_Random` _armcolorlist)))

(event `self.ReceiveActorBeginOverlap`
  (params (OtherActor :type "Actor Object Reference")))

(event `self.Base.OnComponentHit`
  (params (HitComponent :type "PrimitiveComponent Object Reference") (OtherActor :type "Actor Object Reference") (OtherComp :type "PrimitiveComponent Object Reference") (NormalImpulse :type "Vector Structure") (Hit :type "HitResult Structure (by ref)"))
  (`/Engine/EditorBlueprintResources/StandardMacros.DoOnce` false
    (:`Completed`
      (cast `/Game/ThirdPerson/Blueprints/BP_ThirdPersonCharacter_Lo` OtherActor)
      (`GameplayStatics.PlaySound2D` "/Game/StarterContent/Audio/Explosion01.Explosion01" 1.0 1.0 0.0 null null))))

(fn `UserConstructionScript`
  (bind (_coloroptions _snowcolor _armcolor _buttoncolor _snowcolorlist _armcolorlist _buttoncolorlist) (break `/Game/Blueprints/Enums_Structs/Struct_Snowman_Color_Properties` (`self.Color_Properties`)))
  (switch `/Game/Blueprints/Enums_Structs/Enum_Color_Options` _coloroptions
    (:`NewEnumerator0`
      (`PrimitiveComponent.SetMaterial` (`self.Base`) 0 _snowcolor)
      (`PrimitiveComponent.SetMaterial` (`self.Abdomin`) 0 _snowcolor)
      (`PrimitiveComponent.SetMaterial` (`self.Head`) 0 _snowcolor)
      (`PrimitiveComponent.SetMaterial` (`self.Snow_Face2`) 0 _buttoncolor)
      (`PrimitiveComponent.SetMaterial` (`self.Snowman_Buttons`) 0 _buttoncolor)
      (`PrimitiveComponent.SetMaterial` (`self.Snowman_Arms`) 0 _armcolor)
      (`PrimitiveComponent.SetMaterial` (`self.Snowman_Arms1`) 0 _armcolor))
    (:`NewEnumerator1`
      (`PrimitiveComponent.SetMaterial` (`self.Base`) 0 (`KismetArrayLibrary.Array_Random` _snowcolorlist))
      (`PrimitiveComponent.SetMaterial` (`self.Abdomin`) 0 (`KismetArrayLibrary.Array_Random` _snowcolorlist))
      (`PrimitiveComponent.SetMaterial` (`self.Head`) 0 (`KismetArrayLibrary.Array_Random` _snowcolorlist))
      (`PrimitiveComponent.SetMaterial` (`self.Snow_Face2`) 0 (`KismetArrayLibrary.Array_Random` _buttoncolorlist))
      (`PrimitiveComponent.SetMaterial` (`self.Snowman_Buttons`) 0 (`KismetArrayLibrary.Array_Random` _buttoncolorlist))
      (`PrimitiveComponent.SetMaterial` (`self.Snowman_Arms`) 0 (`KismetArrayLibrary.Array_Random` _armcolorlist))
      (`PrimitiveComponent.SetMaterial` (`self.Snowman_Arms1`) 0 (`KismetArrayLibrary.Array_Random` _armcolorlist)))))