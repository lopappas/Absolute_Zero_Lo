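; BP_Platform is a moving platform that shuttles continuously between its starting position and EndLocation.
; BeginPlay stores the relative start location, sets the timeline play rate, then waits for a start delay.
; The TM_Movement timeline lerps the relative location without sweep, pausing for StopDuration at each end before reversing direction.
; The construction script applies a selectable static mesh and material.
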(event `Ev Platform Forward`
  (bind (_direction _alpha) (`Timeline|TM_Movement` :!label _label)
    (:`Update`
      (`SceneComponent.K2_SetRelativeLocation` (`self.Platform`) (`KismetMathLibrary.VLerp` (`self.Starting_Location`) (`self.End_Location`) _alpha) false false))
    (:`Finished`
      (`KismetSystemLibrary.Delay` (`self.Stop_Duration`))
      (if (`|EnumEquality` _direction "Forward")
        (`self.Ev Platform Back`)
        (else
          (`self.Ev Platform Forward`))))))

(event `Ev Platform Back`
  (goto _label :!via `Reverse`))

(event `self.ReceiveBeginPlay`
  (set `self.Starting_Location` (`SceneComponent.RelativeLocation` (`self.Platform`)))
  (`TimelineComponent.SetPlayRate` (`self.TM_Movement`) (`self.Platform_Rate`))
  (`KismetSystemLibrary.Delay` (`self.Start_Delay`))
  (`self.Ev Platform Forward`))

(event `self.ReceiveTick`
  (params (DeltaSeconds :type "Float (single-precision)")))

(fn `UserConstructionScript`
  (`StaticMeshComponent.SetStaticMesh` (`self.Platform`) (`self.SM_Selector`))
  (`PrimitiveComponent.SetMaterial` (`self.Platform`) 0 (`self.Material_Selector`)))