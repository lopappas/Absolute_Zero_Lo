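; BP_Actor_Spawner randomly spawns actors of a configured class at its own transform.
; On BeginPlay it starts a looping timeline at a configurable play rate, used as a per-update tick: each update has a 1-in-221 chance to spawn.
; The volume movement lerp and repeating spawn timer are disconnected, so the spawner stays put and EvSpawnActor does nothing.
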(event `self.ReceiveBeginPlay`
  (bind _tm_spawner_movement (`self.TM_Spawner_Movement`))
  (set `self.Start_Loc` (`SceneComponent.K2_GetComponentLocation` (`self.Spawn_Volume`)))
  (`self.Ev Spawn Actor`)
  (`TimelineComponent.SetPlayRate` _tm_spawner_movement (`self.Play_Rate`))
  (`TimelineComponent.SetLooping` _tm_spawner_movement true)
  (bind (_direction _alpha) (`Timeline|TM_Spawner_Movement`)
    (:`Update`
      (if (== (`KismetMathLibrary.RandomIntegerInRange` 0 220) 100)
        (`|SpawnActorFromClass` (`self.Class`) (`self.GetTransform`) "Undefined" "MultiplyWithRoot" null null)))))

(event `Ev Spawn Actor`)

(fn `UserConstructionScript`)