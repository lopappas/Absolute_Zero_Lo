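; BP_Door is an interactable door that slides between a start and an end location.
; BeginPlay sets the door timeline's play rate from DoorRate.
; InteractPressed toggles InteractState and plays or reverses the timeline, whose Alpha lerps the Door component's relative location without sweep.
; InteractQueried reports the current InteractState to callers.
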(event `self.ReceiveBeginPlay`
  (bind _output_get (set `self.TM_Door_Animation` (`self.TM_Door_Animation`)))
  (`TimelineComponent.SetPlayRate` _output_get (`self.Door Rate`)))

(event `/Game/Blueprints/BPIs/i_Interactable.Interact_Pressed`
  (if (`self.Interact_State`)
    (set `self.Interact_State` false)
    (bind (_direction _alpha) (`Timeline|TM_Door_Animation` :!via `Reverse` :!label _label)
      (:`Update`
        (`SceneComponent.K2_SetRelativeLocation` (`self.Door`) (`KismetMathLibrary.VLerp` (`self.Start_Location`) (`self.End_Location`) _alpha) false false)))
    (else
      (set `self.Interact_State` true)
      (goto _label))))

(fn `Interact_Queried`
  (returns (Trace_Result :type Boolean))
  (return (`self.Interact_State`)))

(fn `UserConstructionScript`)