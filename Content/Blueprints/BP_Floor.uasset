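; BP_Floor is a floor actor that sends the penguin hero back to its spawn when it overlaps the Cube component.
; On begin overlap it casts the other actor to BP_Penguin_Hero and moves it to that character's SpawnLocation without sweep or teleport.
; Hit and overlap events also print debug messages, including the actor name and spawn location.
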(event `self.Cube.OnComponentHit`
  (params (HitComponent :type "PrimitiveComponent Object Reference") (OtherActor :type "Actor Object Reference") (OtherComp :type "PrimitiveComponent Object Reference") (NormalImpulse :type "Vector Structure") (Hit :type "HitResult Structure (by ref)"))
  (`KismetSystemLibrary.PrintString` (`KismetStringLibrary.Concat_StrStr` (`KismetSystemLibrary.GetDisplayName` OtherActor) "  hit us!")))

(event `self.Cube.OnComponentBeginOverlap`
  (params (OverlappedComponent :type "PrimitiveComponent Object Reference") (OtherActor :type "Actor Object Reference") (OtherComp :type "PrimitiveComponent Object Reference") (OtherBodyIndex :type Integer) (bFromSweep :type Boolean) (SweepResult :type "HitResult Structure (by ref)"))
  (`KismetSystemLibrary.PrintString` (`KismetStringLibrary.Concat_StrStr` (`KismetSystemLibrary.GetDisplayName` OtherActor) "  Overlapped us!"))
  (bind _asbp_penguin_hero (cast `/Game/3P_Char_Evans_Tutorial/BP_Penguin_Hero` OtherActor))
  (bind _spawn_location (`/Game/3P_Char_Evans_Tutorial/BP_Penguin_Hero.Spawn_Location` _asbp_penguin_hero))
  (`KismetSystemLibrary.PrintString` (`KismetStringLibrary.Conv_VectorToString` _spawn_location))
  (`self.K2_SetActorLocation` _asbp_penguin_hero _spawn_location false false))

(event `self.Cube.OnComponentEndOverlap`
  (params (OverlappedComponent :type "PrimitiveComponent Object Reference") (OtherActor :type "Actor Object Reference") (OtherComp :type "PrimitiveComponent Object Reference") (OtherBodyIndex :type Integer)))

(fn `UserConstructionScript`)