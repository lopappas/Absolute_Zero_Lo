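; Moving platform that shuttles between its starting location and an end location once EvActivate is called.
; A timeline lerps the Platform component's relative location, reversing after a stop delay at each end while PlayerOn is true.
; The construction script applies a selectable mesh and material.
; Tick and Box overlap events are empty; older tick-based interpolation and overlap-style start/stop logic are disconnected, and BeginPlay's start delay leads nowhere.
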(event `Ev Platform Forward`
  (if (`self.Player_On`)
    (bind (_direction _alpha) (`Timeline|TM_Movement` :!label _label)
      (:`Update`
        (`SceneComponent.K2_SetRelativeLocation` (`self.Platform`) (`KismetMathLibrary.VLerp` (`self.Starting_Location`) (`self.End_Location`) _alpha) false false))
      (:`Finished`
        (if (`|EnumEquality` _direction "Forward")
          (`KismetSystemLibrary.Delay` (`self.Stop_Duration`))
          (`self.Ev Platform Back`)
          (else
            (`KismetSystemLibrary.Delay` (`self.Stop_Duration`))
            (`self.Ev Platform Forward`)))))))

(event `Ev Stop Platform`
  (goto _label :!via `Stop`))

(event `Ev Platform Back`
  (if (`self.Player_On`)
    (goto _label :!via `Reverse`)))

(event `self.ReceiveBeginPlay`
  (set `self.Starting_Location` (`SceneComponent.RelativeLocation` (`self.Platform`)))
  (`TimelineComponent.SetPlayRate` (`self.TM_Movement`) (`self.Platform_Rate`))
  (`KismetSystemLibrary.Delay` (`self.Start_Delay`)))

(event `self.ReceiveTick`
  (params (DeltaSeconds :type "Float (single-precision)"))
  ;[1 1 1] Linear Boomerang Platform using LERP: On every tick, the platform will set itself to the interpolated value's vector (location)
)

(event `self.Box.OnComponentBeginOverlap`
  (params (OverlappedComponent :type "PrimitiveComponent Object Reference") (OtherActor :type "Actor Object Reference") (OtherComp :type "PrimitiveComponent Object Reference") (OtherBodyIndex :type Integer) (bFromSweep :type Boolean) (SweepResult :type "HitResult Structure (by ref)")))

(event `self.Box.OnComponentEndOverlap`
  (params (OverlappedComponent :type "PrimitiveComponent Object Reference") (OtherActor :type "Actor Object Reference") (OtherComp :type "PrimitiveComponent Object Reference") (OtherBodyIndex :type Integer)))

(event `self.Ev Activate`
  (set `self.Player_On` true)
  (`KismetSystemLibrary.Delay` 0.5)
  (`self.Ev Platform Forward`))

(fn `UserConstructionScript`
  (`StaticMeshComponent.SetStaticMesh` (`self.Platform`) (`self.SM_Selector`))
  (`PrimitiveComponent.SetMaterial` (`self.Platform`) 0 (`self.Material_Selector`)))