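; BP_Penny is an interactable penguin actor that plays a sound and hops when the player presses interact.
; A timeline lerps the Penguino2 component from its current world location toward a raised offset along the player capsule's forward vector, applied as relative location.
; A FlipFlop alternates timeline play and reverse, with a Finished flag gating the automatic return.
; InteractQueried returns false, and BeginPlay only prints delta seconds.
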(event `self.ReceiveBeginPlay`
  (`KismetSystemLibrary.PrintString` (`KismetStringLibrary.Conv_DoubleToString` (`GameplayStatics.GetWorldDeltaSeconds`))))

(event `/Game/Blueprints/BPIs/i_Interactable.Interact_Pressed`
  (bind (_forward_vector_x _forward_vector_y _forward_vector_z) (`KismetMathLibrary.BreakVector` (`self.Forward_Vector`)))
  (bind _returnvalue (`SceneComponent.K2_GetComponentLocation` (`self.Penguino2`)))
  (bind _output_get (set `self.Player` (`GameplayStatics.GetPlayerCharacter` 0)))
  (bind _asbp_third_person_character (cast `/Game/ThirdPerson/Blueprints/BP_ThirdPersonCharacter` _output_get))
  (bind (_returnvalue_x _returnvalue_y _returnvalue_z) (`KismetMathLibrary.BreakVector` (`SceneComponent.GetForwardVector` (`Character.CapsuleComponent` _asbp_third_person_character))))
  (set `self.Forward_Vector` (`KismetMathLibrary.MakeVector` _returnvalue_x _returnvalue_y _returnvalue_z))
  (`GameplayStatics.PlaySound2D` "/Game/Sound/SFX/pinguin-220042.pinguin-220042" 1.0 1.0 0.0 null null)
  (`/Engine/EditorBlueprintResources/StandardMacros.FlipFlop` :!label _label
    (:`A`
      (bind (_direction _alpha) (`Timeline|TM_Penguin_Hop` :!label _label_2)
        (:`Update`
          (`SceneComponent.K2_SetRelativeLocation` (`self.Penguino2`) (`KismetMathLibrary.VLerp` _returnvalue (+ _returnvalue (`KismetMathLibrary.MakeVector` (* _forward_vector_x 20.0) (* _forward_vector_y 20.0) (+ _forward_vector_z 30.0))) _alpha) false false))
        (:`Finished`
          (if (`self.Finished`)
            (goto _label_2 :!via `Stop`)
            (else
              (set `self.Finished` true)
              (goto _label))))))
    (:`B`
      (goto _label_2 :!via `Reverse`))))

(fn `Interact_Queried`
  (returns (Trace_Result :type Boolean))
  (return false))

(fn `UserConstructionScript`)