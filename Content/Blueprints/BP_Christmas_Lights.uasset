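; BP_Christmas_Lights is a Christmas lights actor with green, red and yellow light components configured through a LightProperties struct.
; The construction script sets their shared attenuation and scales each bulb's intensity by a Dim, Normal or Bright option.
; On BeginPlay a timeline animates only the green light between its configured intensity and a far brighter multiple, ignoring the selected brightness option.
; The EVFade event is an empty stub.
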(event `self.ReceiveBeginPlay`
  (bind _light_properties (`self.Light Properties`))
  (bind (_direction _alpha) (`Timeline|Timeline`)
    (:`Update`
      (`LightComponent.SetIntensity` (`self.Green_Light`) (`KismetMathLibrary.Lerp` (break `/Game/Blueprints/Structures/Struct_Bulb_Config` (`.BulbConfiguration_10_A43E97284A2BBB1358056591F82E92D5` (break `/Game/Blueprints/Structures/Struct_Light_Properties` _light_properties))) (* (break `/Game/Blueprints/Structures/Struct_Bulb_Config` (`.BulbConfiguration_10_A43E97284A2BBB1358056591F82E92D5` (break `/Game/Blueprints/Structures/Struct_Light_Properties` _light_properties))) 100.0) _alpha)))))

(event `EV Fade`)

(fn `UserConstructionScript`
  (bind (_lightoptions _bulbconfiguration _attenuation) (break `/Game/Blueprints/Structures/Struct_Light_Properties` (`self.Light Properties`)))
  (bind (_greenbulbintensity _redbulbintensity _yellowbulbintensity) (break `/Game/Blueprints/Structures/Struct_Bulb_Config` _bulbconfiguration))
  (`LocalLightComponent.SetAttenuationRadius` (`self.Green_Light`) _attenuation)
  (`LocalLightComponent.SetAttenuationRadius` (`self.Red_Light`) _attenuation)
  (`LocalLightComponent.SetAttenuationRadius` (`self.Yellow_Light`) _attenuation)
  (switch `/Game/Blueprints/Enums_Structs/Enum_Light_Options` _lightoptions
    (:`NewEnumerator0`
      (`LightComponent.SetIntensity` (`self.Green_Light`) (/ _greenbulbintensity 5.0))
      (`LightComponent.SetIntensity` (`self.Red_Light`) (/ _redbulbintensity 5.0))
      (`LightComponent.SetIntensity` (`self.Yellow_Light`) (/ _yellowbulbintensity 5.0)))
    (:`NewEnumerator1`
      (`LightComponent.SetIntensity` (`self.Green_Light`) _greenbulbintensity)
      (`LightComponent.SetIntensity` (`self.Red_Light`) _redbulbintensity)
      (`LightComponent.SetIntensity` (`self.Yellow_Light`) _yellowbulbintensity))
    (:`NewEnumerator2`
      (`LightComponent.SetIntensity` (`self.Green_Light`) (* _greenbulbintensity 3.0))
      (`LightComponent.SetIntensity` (`self.Red_Light`) (* _redbulbintensity 3.0))
      (`LightComponent.SetIntensity` (`self.Yellow_Light`) (* _yellowbulbintensity 3.0)))))