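; Player-controlled third-person penguin character with movement, jumping, fall damage and respawning.
; BeginPlay adds the Enhanced Input mapping context, stores the spawn location and fills health; input events drive movement, invertible camera look and jumps with an intermittent chirp.
; Landing compares downward velocity against three thresholds to set damage and play a whoop sound.
; At zero health, velocity is cleared and the penguin teleports to its spawn with full health.
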(event `self.ReceiveBeginPlay`
  (bind _returnvalue (pcsubsystem `EnhancedInputLocalPlayerSubsystem` (`GameplayStatics.GetPlayerController` 0)))
  (`/Engine/EditorBlueprintResources/StandardMacros.IsValid` _returnvalue
    (:`Is Valid`
      (`KismetSystemLibrary.PrintString` "Controller Success!")
      (`EnhancedInputSubsystemInterface.AddMappingContext` _returnvalue "/Game/3P_Char_Evans_Tutorial/Penguin_Inputs/IMC_Penguin_Third_Person.IMC_Penguin_Third_Person" 0 (struct))
      (set `self.Spawn_Location` (`self.K2_GetActorLocation`))
      (set `self.Health` (`self.Max_Health`)))
    (:`Is Not Valid`
      (`KismetSystemLibrary.PrintString` "Fail to get player controller"))))

(event `self.ReceiveTick`
  (params (DeltaSeconds :type "Float (single-precision)"))
  (if (`NavMovementComponent.IsFalling` (`self.CharacterMovement`))
    _))

(event `EnhancedInput|/Game/3P_Char_Evans_Tutorial/Penguin_Inputs/IA_Penguin_Jump`
  (params (ActionValue :type Boolean) (ElapsedSeconds :type "Float (double-precision)") (TriggeredSeconds :type "Float (double-precision)") (InputAction :type "InputAction Object Reference" :default "/Game/3P_Char_Evans_Tutorial/Penguin_Inputs/IA_Penguin_Jump.IA_Penguin_Jump"))
  ;[0 0.15 0.01905 0.5] Jump controls
  ;;[0 1 0.2685 0.5] Variable jump: Go to class defaults -> "Jump Max Hold Time". and choose a value like .5
  (:`Triggered`
    (`self.Jump`)
    (if (`self.CuteJumpNoise`)
      ;;[0.15 0.0765 0 0.5] every 8 sec your penguin can chirp if it jumps
      (`KismetSystemLibrary.Delay` 8.8)
      (set `self.CuteJumpNoise` false)
      (else
        (`GameplayStatics.PlaySound2D` "/Game/Sound/SFX/pinguin-220042.pinguin-220042" 1.0 1.0 0.0 null null)
        (set `self.CuteJumpNoise` true)))))

(event `EnhancedInput|/Game/3P_Char_Evans_Tutorial/Penguin_Inputs/IA_Penguin_Move_Around`
  (params (ActionValue :type "Vector2D Structure") (ElapsedSeconds :type "Float (double-precision)") (TriggeredSeconds :type "Float (double-precision)") (InputAction :type "InputAction Object Reference" :default "/Game/3P_Char_Evans_Tutorial/Penguin_Inputs/IA_Penguin_Move_Around.IA_Penguin_Move_Around"))
  (bind (_returnvalue_roll _returnvalue_pitch _returnvalue_yaw) (`KismetMathLibrary.BreakRotator` (`self.GetControlRotation`)))
  ; Movement controls
  (:`Triggered`
    ; Left and Right.
    ; Scale Value gets multiplied by max walk speed, and by a + or - depending on action value x, which is either -1 or 1.
    (`self.AddMovementInput` (`KismetMathLibrary.GetRightVector` (`self.GetControlRotation`)) ActionValue_X)
    ; Up and Down
    ; Scale Value gets multiplied by max walk speed, and by a + or - depending on action value x, which is either -1 or 1.
    (`self.AddMovementInput` (`KismetMathLibrary.GetForwardVector` (`KismetMathLibrary.MakeRotator` _returnvalue_roll 0.0 _returnvalue_yaw)) ActionValue_Y)))

(event `EnhancedInput|/Game/3P_Char_Evans_Tutorial/Penguin_Inputs/IA_Penguin_Look_Around`
  (params (ActionValue :type "Vector2D Structure") (ElapsedSeconds :type "Float (double-precision)") (TriggeredSeconds :type "Float (double-precision)") (InputAction :type "InputAction Object Reference" :default "/Game/3P_Char_Evans_Tutorial/Penguin_Inputs/IA_Penguin_Look_Around.IA_Penguin_Look_Around"))
  ; Look Around
  (:`Triggered`
    ; Control player rotation (left & right movement)
    (`self.AddControllerYawInput` (* ActionValue_X (`KismetMathLibrary.SelectFloat` -1.0 1.0 (`self.InvertCameraX`))))
    ; Control player rotation (up & down movement)
    (`self.AddControllerPitchInput` (* ActionValue_Y (`KismetMathLibrary.SelectFloat` -1.0 1.0 (`self.InvertCameraY`))))))

(event `self.OnLanded`
  (params (Hit :type "HitResult Structure (by ref)"))
  (`self.Ev Fall Damage`))

(event `Ev Fall Damage`
  (bind (_returnvalue_x _returnvalue_y _returnvalue_z) (`KismetMathLibrary.BreakVector` (`self.GetVelocity`)))
  (bind (_returnvalue_x_2 _returnvalue_y_2 _returnvalue_z_2) (`KismetMathLibrary.BreakVector` (`self.GetVelocity`)))
  (bind (_returnvalue_x_3 _returnvalue_y_3 _returnvalue_z_3) (`KismetMathLibrary.BreakVector` (`self.GetVelocity`)))
  (bind _returnvalue (* _returnvalue_z_2 -1.0))
  (if (`NavMovementInterface.IsFalling` (`self.CharacterMovement`))
    (`KismetSystemLibrary.PrintString` (`KismetStringLibrary.Conv_DoubleToString` _returnvalue))
    (if (> _returnvalue (`self.FallThreshold1`))
      (if (> (* _returnvalue_z_3 -1.0) (`self.FallThreshold2`))
        (if (> (* _returnvalue_z -1.0) (`self.FallThreshold3`))
          (bind _output_get (set `self.FallDmg` 1.0))
          (set `self.Health` (- (`self.Health`) _output_get))
          (`self.Ev Damage Taken`)
          (`GameplayStatics.PlaySound2D` "/Game/Sound/SFX/6__Close_Whoop.6__Close_Whoop" 1.0 0.5 0.0 null null)
          (else
            (bind _output_get_2 (set `self.FallDmg` 0.66))
            (set `self.Health` (- (`self.Health`) _output_get_2))
            (`GameplayStatics.PlaySound2D` "/Game/Sound/SFX/6__Close_Whoop.6__Close_Whoop" 0.8 0.8 0.0 null null)
            (`self.Ev Damage Taken`)))
        (else
          (bind _output_get_3 (set `self.FallDmg` 0.33))
          (set `self.Health` (- (`self.Health`) _output_get_3))
          (`GameplayStatics.PlaySound2D` "/Game/Sound/SFX/6__Close_Whoop.6__Close_Whoop" 0.8 1.0 0.0 null null)
          (`self.Ev Damage Taken`))))))

(event `self.ReceiveAnyDamage`
  (params (Damage :type "Float (single-precision)") (DamageType :type "DamageType Object Reference") (InstigatedBy :type "Controller Object Reference") (DamageCauser :type "Actor Object Reference")))

(event `Ev Damage Taken`
  (`KismetSystemLibrary.PrintString` (`KismetStringLibrary.Conv_DoubleToString` (`self.Health`)) true true (struct :`G` 0.66 :`B` 1.0 :`A` 1.0) 300.0)
  (if (<= (`self.Health`) 0.0)
    (set `MovementComponent.Velocity` (0.0 0.0 0.0) (`self.CharacterMovement`))
    (`self.K2_SetActorLocation` (`self.Spawn_Location`))
    (set `self.Health` (`self.Max_Health`))
    (`KismetSystemLibrary.PrintString` (`KismetStringLibrary.Conv_DoubleToString` (`self.Health`)))))

(fn `UserConstructionScript`)